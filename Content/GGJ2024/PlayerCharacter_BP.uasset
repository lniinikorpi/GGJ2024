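; Player character for a GGJ2024 game that creates the main HUD and plays a poop-throwing primary effect.
; When ActionComp signals the effect, it spawns a Poop_BP and a timeline scales up its mesh while pinned to the Sphere component.
; A second timeline then slides the Sphere along local X with the poop following its location and rotation, and destroys the poop on finish.
; The throw is purely timeline-driven, with no physics or sweep.
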(event `self.ReceiveBeginPlay`
  (bind _returnvalue (`|CreateWidget` "/Game/GGJ2024/UI/MainHud_Widget.MainHud_Widget_C"))
  (`UserWidget.AddToViewport` _returnvalue 0)
  (add `GActionComponent.OnPlayPrimaryEffect` (`self.ActionComp`) (delegate `OnPlayPrimaryEffect`)))

(event `OnPlayPrimaryEffect`
  (bind _sphere (`self.Sphere`))
  (bind (_relativelocation_x _relativelocation_y _relativelocation_z) (`KismetMathLibrary.BreakVector` (`SceneComponent.RelativeLocation` _sphere)))
  (bind _returnvalue (`|SpawnActorFromClass` "/Game/GGJ2024/MeshBPs/Poop_BP.Poop_BP_C" (`self.GetTransform`) "Undefined" "MultiplyWithRoot" null null))
  (bind (_direction _scaletrack) (`Timeline|PoopScaleTimeline` :!via `PlayFromStart`)
    (:`Update`
      (`SceneComponent.SetWorldScale3D` (`/Game/GGJ2024/MeshBPs/Poop_BP.StaticMesh` _returnvalue) _scaletrack)
      (`self.K2_SetActorLocation` _returnvalue (`SceneComponent.K2_GetComponentLocation` _sphere) false false)
      (`self.K2_SetActorRotation` _returnvalue (`SceneComponent.K2_GetComponentRotation` _sphere) false :!label _label))
    (:`Finished`
      (bind (_direction_2 _position) (`Timeline|ThrowTimeline` :!via `PlayFromStart`)
        (:`Update`
          (`SceneComponent.K2_SetRelativeLocation` _sphere (`KismetMathLibrary.MakeVector` _position _relativelocation_y _relativelocation_z) false false)
          (`self.K2_SetActorLocation` _returnvalue (`SceneComponent.K2_GetComponentLocation` _sphere) false false)
          (goto _label))
        (:`Finished`
          (`self.K2_DestroyActor` _returnvalue))))))

(fn `UserConstructionScript`)