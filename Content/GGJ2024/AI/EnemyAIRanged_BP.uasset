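; Ranged enemy AI Blueprint that procedurally animates its sniper weapon when its primary action effect plays.
; On BeginPlay it binds to the ActionComponent's play-primary-effect event.
; That event runs four chained timelines on SniperParent's relative transform: a shot motion on Y, a roll, a reload motion on Z, then a roll played in reverse.
; Each timeline starts when the previous one finishes.
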(event `self.ReceiveBeginPlay`
  (add `GActionComponent.OnPlayPrimaryEffect` (`self.ActionComponent`) (delegate `OnPlayPrimaryEffect`)))

(event `OnPlayPrimaryEffect`
  (bind _sniperparent (`self.SniperParent`))
  (bind _sniperparent_2 (`self.SniperParent`))
  (bind _sniperparent_3 (`self.SniperParent`))
  (bind _sniperparent_4 (`self.SniperParent`))
  (bind (_relativelocation_x _relativelocation_y) (`KismetMathLibrary.BreakVector` (`SceneComponent.RelativeLocation` _sniperparent)))
  (bind (_relativerotation_roll _relativerotation_pitch _relativerotation_yaw) (`KismetMathLibrary.BreakRotator` (`SceneComponent.RelativeRotation` _sniperparent_2)))
  (bind (_relativelocation_x_2 _relativelocation_y_2 _relativelocation_z) (`KismetMathLibrary.BreakVector` (`SceneComponent.RelativeLocation` _sniperparent_3)))
  (bind (_relativerotation_roll_2 _relativerotation_pitch_2 _relativerotation_yaw_2) (`KismetMathLibrary.BreakRotator` (`SceneComponent.RelativeRotation` _sniperparent_4)))
  (bind (_direction _position) (`Timeline|ShootTimeline` :!via `PlayFromStart`)
    (:`Update`
      (`SceneComponent.K2_SetRelativeLocation` _sniperparent_3 (`KismetMathLibrary.MakeVector` _relativelocation_x_2 _position _relativelocation_z) false false))
    (:`Finished`
      (bind (_direction_2 _rotation) (`Timeline|RotationTimeline` :!via `PlayFromStart`)
        (:`Update`
          (`SceneComponent.K2_SetRelativeRotation` _sniperparent_4 (`KismetMathLibrary.MakeRotator` _rotation _relativerotation_pitch_2 _relativerotation_yaw_2) false false))
        (:`Finished`
          (bind (_direction_3 _position_2) (`Timeline|ReloadTimeline` :!via `PlayFromStart`)
            (:`Update`
              (`SceneComponent.K2_SetRelativeLocation` _sniperparent (`KismetMathLibrary.MakeVector` _relativelocation_x _relativelocation_y _position_2) false false))
            (:`Finished`
              (bind (_direction_4 _rotation_2) (`Timeline|RotationTImelineInverse` :!via `ReverseFromEnd`)
                (:`Update`
                  (`SceneComponent.K2_SetRelativeRotation` _sniperparent_2 (`KismetMathLibrary.MakeRotator` _rotation_2 _relativerotation_pitch _relativerotation_yaw) false false))))))))))

(fn `UserConstructionScript`)